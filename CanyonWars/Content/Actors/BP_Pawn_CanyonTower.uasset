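; BP_Pawn_CanyonTower is a player-controlled cannon turret pawn that fires projectiles and can be destroyed by damage.
; Forward input pitches the cannon, while Right input yaws the base platform and copies that yaw to the first-person camera.
; Shoot spawns a BP_Proyectile at the muzzle transform, and V toggles between first-person and aerial cameras.
; AnyDamage subtracts from Vida, printing debug messages and destroying the tower when health runs out.
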(event EventBeginPlay)

(event Collision|EventActorBeginOverlap
  (params (OtherActor :type Actor%20Object%20Reference)))

(event EventTick
  (params (DeltaSeconds :type Float%20%28single-precision%29)))

(event Game|Damage|EventAnyDamage
  (params (Damage :type Float%20%28single-precision%29) (DamageType :type Damage%20Type%20Object%20Reference) (InstigatedBy :type Controller%20Object%20Reference) (DamageCauser :type Actor%20Object%20Reference))
  (Development|PrintString "Daño inflingido")
  (Variables|Default|SetVida (- (Variables|Default|GetVida) Damage))
  (if (<= (Variables|Default|GetVida) 0.0)
    (Development|PrintString "Torre Destruida")
    (Actor|DestroyActor)))

(event Input|ActionEvents|InputActionInputAction_PressV
  (params (Key :type Key%20Structure :default "None"))
  (:Pressed
    (Utilities|FlowControl|FlipFlop
      (:A
        (Components|Activation|SetActive (Variables|Default|GetCameraFirstPerson) true false)
        (Components|Activation|SetActive (Variables|Default|GetCamaraAerea) false false))
      (:B
        (Components|Activation|SetActive (Variables|Default|GetCamaraAerea) true false)
        (Components|Activation|SetActive (Variables|Default|GetCameraFirstPerson) false false)))))

(event Input|ActionEvents|InputActionInputAction_Shoot
  (params (Key :type Key%20Structure :default "None"))
  (bind _direccionbala (Variables|Default|GetDireccionBala))
  (bind _returnvalue (Transformation|GetWorldTransform _direccionbala))
  (:Pressed
    (bind _returnvalue_2 (Game|SpawnActorfromClass "/Game/Actors/BP_Proyectile.BP_Proyectile_C" (Math|Transform|MakeTransform (.location _returnvalue) (.rotation _returnvalue) "1.000000,1.000000,1.000000") "AlwaysSpawn" "MultiplyWithRoot" 0 0))))

(event Input|AxisEvents|InputAxisInputAxis_Right
  (params (AxisValue :type Float%20%28single-precision%29))
  (bind _camerafirstperson (Variables|Default|GetCameraFirstPerson))
  (bind _returnvalue (Transformation|GetSocketRotation _camerafirstperson "None"))
  (if (!= AxisValue 0.0)
    (Transformation|AddRelativeRotation (Variables|Default|GetPlataformaBase) (Math|Rotator|MakeRotator 0.0 0.0 (* AxisValue 0.2)) false false)
    (Transformation|SetRelativeRotation _camerafirstperson (Math|Rotator|MakeRotator (.roll _returnvalue) (.pitch _returnvalue) (.yaw (Transformation|GetSocketRotation (Variables|Default|GetPlataformaBase) "None"))) false false)))

(event Input|AxisEvents|InputAxisInputAxis_Forward
  (params (AxisValue :type Float%20%28single-precision%29))
  (if (!= AxisValue 0.0)
    (Transformation|AddRelativeRotation (Variables|Default|GetDireccionCannon) (Math|Rotator|MakeRotator 0.0 (* AxisValue 0.2) 0.0) false false)))

(fn ConstructionScript)